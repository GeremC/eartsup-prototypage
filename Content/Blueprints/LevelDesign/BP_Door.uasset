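; BP_Door is a level design door that slides vertically open and closed.
; On BeginPlay it caches the DoorMesh world location as the closed position.
; OpenDoor plays a Timeline whose track lerps the mesh up to a fixed height above that position, without sweep.
; CloseDoor reverses the same Timeline; both are custom events with no trigger logic in this Blueprint.
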(event `self.ReceiveBeginPlay`
  (set `self.InitialLocation` (`SceneComponent.K2_GetComponentLocation` (`self.DoorMesh`))))

(event `self.OpenDoor`
  (bind (_initiallocation_x _initiallocation_y _initiallocation_z) (`KismetMathLibrary.BreakVector` (`self.InitialLocation`)))
  (bind (_direction _newtrack_0) (`Timeline|Timeline` :!label _label)
    (:`Update`
      (`SceneComponent.K2_SetWorldLocation` (`self.DoorMesh`) (`KismetMathLibrary.VLerp` (`self.InitialLocation`) (`KismetMathLibrary.MakeVector` _initiallocation_x _initiallocation_y (+ _initiallocation_z 300.0)) _newtrack_0) false false))))

(event `self.CloseDoor`
  (goto _label :!via `Reverse`))

(fn `UserConstructionScript`)